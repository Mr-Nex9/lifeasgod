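; Map tile actor for a generated map, showing one square or hexagon cell as terrain.
; Initialize picks the mesh, attaches to the owner and offsets the tile by row and column, staggering hex rows.
; SetTileInfo derives landscape from height and land flag, then sets color, surface parameters and Z scale for elevation.
; A dynamic material instance drives all tinting, including river, desert, forest and selection highlight colors.
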(event EventBeginPlay
  (Main|CreateMID))

(event Collision|EventActorBeginOverlap
  (params (OtherActor :type Actor%20Object%20Reference)))

(event EventTick
  (params (DeltaSeconds :type Float%20%28single-precision%29)))

(fn ConstructionScript)

(fn Initialize
  (params (In_Type :type E_GridType%20Enum :default "NewEnumerator0"))
  (bind _returnvalue (Components|GetOwner))
  (Utilities|IsValid _returnvalue
    (:Is%20Valid
      (Main|SetMesh In_Type)
      (Transformation|AttachActorToActor _returnvalue "None" "SnapToTarget" "SnapToTarget" "KeepRelative" false)
      (bind _location (Main|CalculateLocation In_Type))
      (Transformation|SetActorRelativeLocation _location))))

(fn SetMesh
  (params (In_Type :type E_GridType%20Enum :default "NewEnumerator0"))
  (Components|StaticMesh|SetStaticMesh (Variables|Default|GetTile) (Utilities|Select :Index In_Type :NewEnumerator0 "/Engine/BasicShapes/Plane.Plane" :NewEnumerator1 "/Game/Meshes/HexTile2_Flat.HexTile2_Flat"))
  (Main|CreateMID))

(fn CalculateLocation
  (params (Type :type E_GridType%20Enum :default "NewEnumerator0"))
  (bind _tile (Variables|Default|GetTile))
  (bind _column (Variables|MapGen|GetColumn))
  (bind _boxextent (Collision|GetComponentBounds _tile))
  (bind (_x _y) (Math|Vector|BreakVector _boxextent))
  (bind _returnvalue (* _x 2.0 _column))
  (return (Utilities|Select :Index Type :NewEnumerator0 (Math|Vector|MakeVector (* _x 2.0 (Variables|MapGen|GetRow)) (* _y 2.0 (Variables|MapGen|GetColumn)) 0.0) :NewEnumerator1 (Math|Vector|MakeVector (* _y 2.0 (Variables|MapGen|GetRow) (/ 3.0 4.0)) (Math|Float|SelectFloat _returnvalue (+ _returnvalue _x) (== (Math|Integer|%(Integer) (Variables|MapGen|GetRow) 2) 0)) 0.0))))

(fn CreateMID
  (bind _returnvalue (Rendering|Material|CreateDynamicMaterialInstance (Variables|Default|GetTile) 0 "/Game/Materials/M_Tile.M_Tile" "None" :!class /Script/Engine.PrimitiveComponent))
  (bind _output_get (Variables|Color|SetMID _returnvalue))
  (Rendering|Material|SetVectorParameterValue :self _output_get :ParameterName "Color" :!class /Script/Engine.MaterialInstanceDynamic))

(fn SetTileInfo
  (params (In_Height :type Float%20%28double-precision%29) (In_IsLand? :type Boolean))
  (bind _mapdata (Variables|MapGen|GetMapData))
  (Utilities|Struct|SetmembersinBPS_TileMapData (Variables|MapGen|GetMapData) In_Height In_IsLand?)
  (Info|SetRegionInfo)
  (Info|SetDefaultColor)
  (if (.island? (Variables|MapGen|GetMapData))
    (Transformation|SetActorScale3D (Math|Vector|MakeVector 1.0 1.0 (* (.height _mapdata) (Utilities|Select :Index (.landscape _mapdata) :NewEnumerator0 2.0 :NewEnumerator1 1e+01 :NewEnumerator2 15.0 :NewEnumerator3 2e+01 :NewEnumerator4 0.0))))
    (else
      (Transformation|SetActorScale3D (Math|Vector|MakeVector 1.0 1.0 1.0)))))

(fn SetDefaultColor
  (bind _mapdata (Variables|MapGen|GetMapData))
  (bind _mapdata_2 (Variables|MapGen|GetMapData))
  (bind _returnvalue (Utilities|Select :Index (.landscape _mapdata) :NewEnumerator0 "(R=0.000000,G=0.027321,B=0.234551,A=1.000000)" :NewEnumerator1 "(R=0.000000,G=0.098958,B=0.001560,A=1.000000)" :NewEnumerator2 "(R=0.017529,G=0.062500,B=0.000000,A=1.000000)" :NewEnumerator3 "(R=0.125490,G=0.125490,B=0.125490,A=1.000000)" :NewEnumerator4 ""))
  (Rendering|Material|SetVectorParameterValue (Variables|Color|GetMID) "Color" _returnvalue :!class /Script/Engine.MaterialInstanceDynamic)
  (Variables|Color|SetDefaultColor _returnvalue)
  (Rendering|Material|SetScalarParameterValue (Variables|Color|GetMID) "Roughness" (Math|Float|SelectFloat 0.9 0.2 (.island? _mapdata_2)) :!class /Script/Engine.MaterialInstanceDynamic)
  (Rendering|Material|SetScalarParameterValue (Variables|Color|GetMID) "Metallic" (Math|Float|SelectFloat 0.0 0.5 (.island? _mapdata_2)) :!class /Script/Engine.MaterialInstanceDynamic))

(fn SetRegionInfo
  (|SetHeightData))

(fn SetRiverColor
  (Rendering|Material|SetVectorParameterValue (Variables|Color|GetMID) "Color" (Utilities|Select :Index (.landscape (Variables|MapGen|GetMapData)) :NewEnumerator0 "(R=0.000000,G=0.027321,B=0.234551,A=1.000000)" :NewEnumerator1 "(R=0.000000,G=0.098958,B=0.001560,A=1.000000)" :NewEnumerator2 "(R=0.017529,G=0.062500,B=0.000000,A=1.000000)" :NewEnumerator3 "(R=0.125490,G=0.125490,B=0.125490,A=1.000000)" :NewEnumerator4 "(R=0.000000,G=0.035243,B=0.302083,A=1.000000)") :!class /Script/Engine.MaterialInstanceDynamic))

(fn SetDesertColor
  (if (.isdesert? (Variables|MapGen|GetMapData))
    (Rendering|Material|SetVectorParameterValue (Variables|Color|GetMID) "Color" (Utilities|Select :Index (.climate (Variables|MapGen|GetMapData)) :NewEnumerator0 "(R=0.396078,G=0.305882,B=0.105882,A=1.000000)" :NewEnumerator2 "" :NewEnumerator3 "" :NewEnumerator4 "(R=1.000000,G=1.000000,B=1.000000,A=1.000000)") :!class /Script/Engine.MaterialInstanceDynamic)
    (elif (Utilities|Enum|Equal(Enum) (.climate (Variables|MapGen|GetMapData)) "NewEnumerator4")
      (Rendering|Material|SetVectorParameterValue (Variables|Color|GetMID) "Color" "(R=0.770833,G=0.770833,B=0.770833,A=1.000000)" :!class /Script/Engine.MaterialInstanceDynamic))))

(fn SetForestCOlor
  (Rendering|Material|SetVectorParameterValue (Variables|Color|GetMID) "Color" (Utilities|Select :Index (.landscape (Variables|MapGen|GetMapData)) :NewEnumerator0 "(R=0.000000,G=0.027321,B=0.234551,A=1.000000)" :NewEnumerator1 "(R=0.011720,G=0.041667,B=0.000000,A=1.000000)" :NewEnumerator2 "(R=0.010253,G=0.036458,B=0.000000,A=1.000000)" :NewEnumerator3 "(R=0.125490,G=0.125490,B=0.125490,A=1.000000)" :NewEnumerator4 "") :!class /Script/Engine.MaterialInstanceDynamic))

(fn OnInteract
  (params (bIn_Selected :type Boolean))
  (bind _mid (Variables|Color|GetMID)
    (:then
      (Rendering|Material|SetVectorParameterValue _mid "Color" (Math|Color|SelectColor (Variables|Color|GetSelectedColor) (Variables|Color|GetDefaultColor) bIn_Selected) :!class /Script/Engine.MaterialInstanceDynamic)
      (return true))
    (:else
      (return false))))