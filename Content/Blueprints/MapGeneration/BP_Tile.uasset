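; BP_Tile is a single map-generation tile, shown as either land or water on a square or hexagonal grid.
; Initialize, given a valid owner, picks the plane or hex mesh, attaches to that owner, and colors the tile green for land or blue otherwise.
; CalculateLocation derives the relative position from Row, Column and mesh bounds, spacing hex columns at three-quarter width and shifting odd columns half a tile.
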(event EventBeginPlay)

(event Collision|EventActorBeginOverlap
  (params (OtherActor :type Actor%20Object%20Reference)))

(event EventTick
  (params (DeltaSeconds :type Float%20%28single-precision%29)))

(fn ConstructionScript)

(fn Initialize
  (params (In_Type :type E_GridType%20Enum :default "NewEnumerator0") (In_IsLand? :type Boolean))
  (bind _returnvalue (Components|GetOwner))
  (Variables|Default|SetIsLand? In_IsLand?)
  (Utilities|IsValid _returnvalue
    (:Is%20Valid
      (CallFunction|SetMesh In_Type)
      (Transformation|AttachActorToActor _returnvalue "None" "SnapToTarget" "SnapToTarget" "KeepRelative" false)
      (bind _location (CallFunction|CalculateLocation In_Type))
      (Transformation|SetActorRelativeLocation _location)
      (Rendering|Material|SetMaterial (Variables|Default|GetTile) 0 (select (Variables|Default|GetIsLand?) "/Game/Materials/M_Green.M_Green" "/Game/Materials/M_Blue.M_Blue")))))

(fn SetMesh
  (params (In_Type :type E_GridType%20Enum :default "NewEnumerator0"))
  (Components|StaticMesh|SetStaticMesh (Variables|Default|GetTile) (Utilities|Select :Index In_Type :NewEnumerator0 "/Engine/BasicShapes/Plane.Plane" :NewEnumerator1 "/Game/Meshes/HexTile_Flat.HexTile_Flat")))

(fn CalculateLocation
  (params (Type :type E_GridType%20Enum :default "NewEnumerator0"))
  (bind _tile (Variables|Default|GetTile))
  (bind _row (Variables|Default|GetRow))
  (bind _boxextent (Collision|GetComponentBounds _tile))
  (bind (_x _y) (Math|Vector|BreakVector _boxextent))
  (bind _returnvalue (* _y 2.0 _row))
  (return (Utilities|Select :Index Type :NewEnumerator0 (Math|Vector|MakeVector (* _x 2.0 (Variables|Default|GetColumn)) (* _y 2.0 (Variables|Default|GetRow)) 0.0) :NewEnumerator1 (Math|Vector|MakeVector (* _x 2.0 (Variables|Default|GetColumn) (/ 3.0 4.0)) (Math|Float|SelectFloat _returnvalue (+ _returnvalue _y) (== (Math|Integer|%(Integer) (Variables|Default|GetColumn) 2) 0)) 0.0))))